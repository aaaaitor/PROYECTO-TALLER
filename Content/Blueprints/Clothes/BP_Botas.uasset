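; BP_Botas is a boots ("botas") clothing pickup that a VR player can take.
; Every Tick rotates the actor slightly and drives two timelines, one forward and one in reverse, that apply local offsets to the two meshes.
; A box overlap with VRPawn toggles CanGrab, and TakeBotas destroys the actor when that flag is set.
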(event `self.ReceiveTick`
  (params (DeltaSeconds :type "Float (single-precision)"))
  (`self.K2_SetActorRotation` (`KismetMathLibrary.ComposeRotators` (`self.K2_GetActorRotation`) (struct :`Yaw` 0.1)))
  (`|ExecutionSequence`
    (:`then_0`
      (bind (_direction _newtrack_1) (`Timeline|Timeline`)
        (:`Update`
          (`SceneComponent.K2_AddLocalOffset` (`self.StaticMesh`) _newtrack_1 false false))))
    (:`then_1`
      (bind (_direction_2 _newtrack_1_2) (`Timeline|Timeline_0` :!via `Reverse`)
        (:`Update`
          (`SceneComponent.K2_AddLocalOffset` (`self.StaticMesh1`) _newtrack_1_2 false false))))))

(event `self.Box.OnComponentBeginOverlap`
  (params (OverlappedComponent :type "PrimitiveComponent Object Reference") (OtherActor :type "Actor Object Reference") (OtherComp :type "PrimitiveComponent Object Reference") (OtherBodyIndex :type Integer) (bFromSweep :type Boolean) (SweepResult :type "HitResult Structure (by ref)"))
  ;[1 1 1] Check if hand is in grab area
  (cast `/Game/VRTemplate/Blueprints/VRPawn` OtherActor)
  (set `self.bCanGrab` true))

(event `self.Box.OnComponentEndOverlap`
  (params (OverlappedComponent :type "PrimitiveComponent Object Reference") (OtherActor :type "Actor Object Reference") (OtherComp :type "PrimitiveComponent Object Reference") (OtherBodyIndex :type Integer))
  ;[1 1 1] Check if hand is in grab area
  (cast `/Game/VRTemplate/Blueprints/VRPawn` OtherActor)
  (set `self.bCanGrab` false))

(event `TakeBotas`
  ;[1 1 1] If actor is grabbed destroy itself
  (if (`self.bCanGrab`)
    (`self.K2_DestroyActor`)))

(fn `UserConstructionScript`)