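; BP_Boton is a pressable button that reacts when a VRPawn overlaps its Colision component.
; On overlap it slides the Boton component down from its BeginPlay position, sets IsPressed and plays a click sound at the world origin, guarded by AudioPlayed.
; When the overlap ends it slides back and re-arms the sound, while IsPressed stays true.
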(event `self.ReceiveBeginPlay`
  ;[1 1 1] Guarda la posicion del boton al empezar el juego
  (set `self.ButtonStart` (`SceneComponent.RelativeLocation` (`self.boton`))))

(event `self.colision.OnComponentBeginOverlap`
  (params (OverlappedComponent :type "PrimitiveComponent Object Reference") (OtherActor :type "Actor Object Reference") (OtherComp :type "PrimitiveComponent Object Reference") (OtherBodyIndex :type Integer) (bFromSweep :type Boolean) (SweepResult :type "HitResult Structure (by ref)"))
  ;[1 1 1] Mueve el boton dependiendo de si se esta pulsando o soltando
  (cast `/Game/VRTemplate/Blueprints/VRPawn` OtherActor)
  (`KismetSystemLibrary.MoveComponentTo` (`self.boton`) (- (`self.ButtonStart`) (0.0 0.0 5.0)) (struct) false false 0.1)
  (set `self.IsPressed` true)
  (if (not (`self.bAudioPlayed`))
    (`GameplayStatics.PlaySoundAtLocation` "/Game/Audio/SFX/SFX_boton.SFX_boton" (0.0 0.0 0.0) (struct) 1.0 1.0 0.0 null null null null)
    (set `self.bAudioPlayed` true)))

(event `self.colision.OnComponentEndOverlap`
  (params (OverlappedComponent :type "PrimitiveComponent Object Reference") (OtherActor :type "Actor Object Reference") (OtherComp :type "PrimitiveComponent Object Reference") (OtherBodyIndex :type Integer))
  ;[1 1 1] Mueve el boton dependiendo de si se esta pulsando o soltando
  (cast `/Game/VRTemplate/Blueprints/VRPawn` OtherActor)
  (`KismetSystemLibrary.MoveComponentTo` (`self.boton`) (`self.ButtonStart`) (struct) false false 0.1)
  (set `self.bAudioPlayed` false))

(fn `UserConstructionScript`)