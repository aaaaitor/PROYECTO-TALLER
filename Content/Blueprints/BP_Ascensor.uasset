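; VR elevator actor that drives two sliding doors, sounds and player teleport permission from two child-actor buttons.
; BeginPlay caches both doors' relative transforms as their starting positions.
; Tick polls the buttons: the first alone plays travel audio and a ping, then slides the doors apart.
; With both pressed, doors return to start, VRPawn teleporting is enabled, and delayed music plays, a step marked as development placeholder.
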(event `self.ReceiveBeginPlay`
  ;[1 1 1] Asigna la posicion y rotacion de las puertas.
  (`self.GetDoorPosRotInWorld`))

(event `self.ReceiveTick`
  (params (DeltaSeconds :type "Float (single-precision)"))
  (bind _p1location (`self.P1Location`))
  ;[1 1 1] Si el boton es pulsado mueve las puertas a una posicion especifica.
  (bind _asbp_boton_ascensor (cast `/Game/Blueprints/BP_BotonAscensor` (`ChildActorComponent.ChildActor` (`self.BP_BotonAscensor1`))))
  (if (`/Game/Blueprints/BP_BotonAscensor.IsPressed` _asbp_boton_ascensor)
    (bind _asbp_boton_ascensor_2 (cast `/Game/Blueprints/BP_BotonAscensor` (`ChildActorComponent.ChildActor` (`self.BP_BotonAscensor`))))
    (if (`/Game/Blueprints/BP_BotonAscensor.IsPressed` _asbp_boton_ascensor_2)
      (bind _asvrpawn (cast `/Game/VRTemplate/Blueprints/VRPawn` (`GameplayStatics.GetPlayerPawn` 0)))
      (set `/Game/VRTemplate/Blueprints/VRPawn.bCanTeleport` true _asvrpawn)
      (`|ExecutionSequence`
        (:`then_0`
          (`KismetSystemLibrary.MoveComponentTo` (`self.puerta1`) (`self.P1Location`) (`self.P1Rotation`) false false 0.4))
        (:`then_1`
          (`KismetSystemLibrary.MoveComponentTo` (`self.puerta2`) (`self.P2Location`) (`self.P2Rotation`) false false 0.4))
        (:`then_2`
          ;[1 1 1] DEVELOPMENT, HAS TO BE CHANGED
          (if (not (`self.bElevatorMusicPlayed`))
            (`KismetSystemLibrary.Delay` 3.0)
            (`GameplayStatics.PlaySoundAtLocation` "/Game/Audio/MUSICA/AU_elevator_music_local-forecast-slower-by-kevin-macleod-from-filmmusic-io.AU_elevator_music_local-forecast-slower-by-kevin-macleod-from-filmmusic-io" (0.0 0.0 0.0) (struct) 0.3 1.0 0.0 null null null null)
            (set `self.bElevatorMusicPlayed` true))))
      (elif (not (`self.bElevatorRunningAudioPlayed`))
        (set `self.bElevatorRunningAudioPlayed` true)
        (`GameplayStatics.PlaySoundAtLocation` "/Game/Audio/SFX/SFX_ascensor_camino.SFX_ascensor_camino" _p1location (struct) 1.0 1.0 0.0 null null null null)
        (`KismetSystemLibrary.Delay` 8.4)
        (`GameplayStatics.PlaySoundAtLocation` "/Game/Audio/SFX/SFX_ping_ascensor.SFX_ping_ascensor" _p1location (struct) 1.0 1.0 0.0 null null null null)
        (`|ExecutionSequence`
          (:`then_0`
            (`KismetSystemLibrary.MoveComponentTo` (`self.puerta1`) (+ (`self.P1Location`) (-65.0 0.0 0.0)) (`self.P1Rotation`) false false 0.4))
          (:`then_1`
            (`KismetSystemLibrary.MoveComponentTo` (`self.puerta2`) (+ (`self.P2Location`) (65.0 0.0 0.0)) (`self.P2Rotation`) false false 0.4)))))))

(fn `GetDoorPosRotInWorld`
  (bind _puerta1 (`self.puerta1`))
  (bind _puerta2 (`self.puerta2`))
  ;[1 1 1] Recoge y guarda la posicion y rotacion de cada puerta del ascensor cuando se incia el blueprint para poder mover la puerta mas tarde.
  (set `self.P1Location` (`SceneComponent.RelativeLocation` _puerta1))
  (set `self.P1Rotation` (`SceneComponent.RelativeRotation` _puerta1))
  (set `self.P2Location` (`SceneComponent.RelativeLocation` _puerta2))
  (set `self.P2Rotation` (`SceneComponent.RelativeRotation` _puerta2)))

(fn `UserConstructionScript`)