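; Trigger actor that plays a sound once when the VRPawn overlaps its box, with timed subtitles on the pawn.
; An AudioPlayed flag blocks replays, and the sound plays at the box's relative location.
; A loop over the Subtitles map keys sets and clears the pawn's text around a map-timed Delay.
; As wired, text and lookup key are empty strings, and the loop does not wait for the Delay.
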(event `self.Box.OnComponentBeginOverlap`
  (params (OverlappedComponent :type "PrimitiveComponent Object Reference") (OtherActor :type "Actor Object Reference") (OtherComp :type "PrimitiveComponent Object Reference") (OtherBodyIndex :type Integer) (bFromSweep :type Boolean) (SweepResult :type "HitResult Structure (by ref)"))
  (bind _subtitles (`self.Subtitles`))
  ;[1 1 1] Ejecuta un archivo de audio seleccionado en el nodo de play sound location cuando se hace overlap con el trigger.
  (bind _asvrpawn (cast `/Game/VRTemplate/Blueprints/VRPawn` OtherActor))
  (if (not (`self.AudioPlayed`))
    (`GameplayStatics.PlaySoundAtLocation` (`self.Sound`) (`SceneComponent.RelativeLocation` OverlappedComponent) (struct) 1.0 1.0 0.0 null null null null)
    (set `self.AudioPlayed` true)
    ;[1 1 1] actualiza el texto de los subtitlos durante un tiempo especifico y pasado ese tiempo los limpia de la pantalla
    (bind _keys (`BlueprintMapLibrary.Map_Keys` _subtitles))
    (for _ (range (`self.Index`) (+ (`KismetArrayLibrary.Array_Length` _keys) 1))
      (bind _subtitles_2 (`/Game/VRTemplate/Blueprints/VRPawn.Subtitles` _asvrpawn))
      (`TextRenderComponent.K2_SetText` _subtitles_2 (`KismetTextLibrary.Conv_StringToText` ""))
      (`KismetSystemLibrary.Delay` (`BlueprintMapLibrary.Map_Find` _subtitles))
      (`TextRenderComponent.K2_SetText` _subtitles_2 (`self.EmptyText`))
      (bind _result (`/Engine/EditorBlueprintResources/StandardMacros.IncrementInt` (`self.Index`))
        (:`  `
          (set `self.Index` _result))))))

(fn `UserConstructionScript`)